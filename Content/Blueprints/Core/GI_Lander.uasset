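; GI_Lander is the Lander game's GameInstance, holding persistent progress: levels, completed levels, wins and deaths.
; On Init it loads the "Lander" save slot, or creates a new Save_Lander object and writes it if none exists.
; LoadGame and SaveGame copy values between the instance and the save object.
; Death and Win events increment their counters and save immediately.
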(event Custom|Load%20Game
  ;[1 1 1] Load saved info
  (bind _assave_lander (Utilities|Casting|CastToSave_Lander (Variables|Default|GetSave%20Ref)))
  (Variables|Default|SetLevels (Variables|/Game/Blueprints/Core/Save_Lander.Save_Lander_C|GetLevels _assave_lander))
  (Variables|Default|SetLevels%20Complete (Variables|/Game/Blueprints/Core/Save_Lander.Save_Lander_C|GetLevels%20Complete _assave_lander))
  (Variables|Default|SetWins (Variables|/Game/Blueprints/Core/Save_Lander.Save_Lander_C|GetWins _assave_lander))
  (Variables|Default|SetDeaths (Variables|/Game/Blueprints/Core/Save_Lander.Save_Lander_C|GetDeaths _assave_lander)))

(event Custom|Save%20Game
  ;[1 1 1] Update save game
  (bind _assave_lander (Utilities|Casting|CastToSave_Lander (Variables|Default|GetSave%20Ref)))
  (Variables|/Game/Blueprints/Core/Save_Lander.Save_Lander_C|SetLevels _assave_lander (Variables|Default|GetLevels))
  (Variables|/Game/Blueprints/Core/Save_Lander.Save_Lander_C|SetLevels%20Complete _assave_lander (Variables|Default|GetLevels%20Complete))
  (Variables|/Game/Blueprints/Core/Save_Lander.Save_Lander_C|SetDeaths _assave_lander (Variables|Default|GetDeaths))
  (Variables|/Game/Blueprints/Core/Save_Lander.Save_Lander_C|SetWins _assave_lander (Variables|Default|GetWins))
  (SaveGame|SaveGametoSlot (Variables|Default|GetSave%20Ref) "Lander"))

(event Custom|Win
  (Math|Integer|IncrementInt (Variables|Default|GetWins)
    (:%20%20
      (CallFunction|SaveGame))))

(event Custom|Death
  (Math|Integer|IncrementInt (Variables|Default|GetDeaths)
    (:%20%20
      (CallFunction|SaveGame))))

(event EventInit
  (bind _returnvalue (SaveGame|DoesSaveGameExist "Lander"))
  (if _returnvalue
    (bind _returnvalue_2 (SaveGame|LoadGamefromSlot "Lander"))
    (Variables|Default|SetSave%20Ref _returnvalue_2)
    (CallFunction|LoadGame)
    (else
      (bind _returnvalue_3 (SaveGame|CreateSaveGameObject "/Game/Blueprints/Core/Save_Lander.Save_Lander_C"))
      (Variables|Default|SetSave%20Ref _returnvalue_3)
      (CallFunction|SaveGame))))