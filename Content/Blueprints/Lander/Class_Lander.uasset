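; Player-controlled lander with physics-driven flight, limited fuel and an optional 3D mode; outside 3D it allows only roll and pins the mesh to the X=0 plane.
; Axis or held-button input sets a target thrust, which is interpolated each Tick into upward force while the camera stays upright.
; A looping timer burns fuel by current thrust, RecieveFuel refills it, and hits above a speed tolerance only print a death message.
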(event EventBeginPlay
  (CallFunction|StartFuelUse)
  (Class|PrimitiveComponent|SetAngularDamping (Variables|Default|GetStaticMesh) 0.1))

(event EventTick
  (params (DeltaSeconds :type Float%20%28single-precision%29))
  (bind _staticmesh (Variables|Default|GetStaticMesh))
  (bind _camera (Variables|Default|GetCamera))
  (bind _returnvalue (Transformation|GetWorldLocation _staticmesh))
  (CallFunction|MainThrust)
  (Transformation|SetWorldRotation _camera (Math|Rotator|MakeRotfromXZ (Math|Vector|GetForwardVector _camera) (Math|Vector|MakeVector 0.0 0.0 1.0)) false false)
  (if (not (Variables|Default|GetIs%203D?))
    (Transformation|SetWorldLocation _staticmesh (Math|Vector|MakeVector 0.0 (.y _returnvalue) (.z _returnvalue)) false false)))

(event Custom|Main%20Thrust
  ;[1 1 1] Thrust Solver
  (if (Variables|Default|GetHas%20Fuel)
    (bind _output_get (Variables|Thrust|SetCurrent%20Thrust (Math|Interpolation|FInterpTo (Variables|Thrust|GetCurrent%20Thrust) (Math|Float|Clamp(Float) (Variables|Thrust|GetTarget%20Thrust)) (Variables|Default|GetInterp%20Delta) (Variables|Default|GetInterp%20Speed))))
    (Physics|AddForce (Variables|Default|GetStaticMesh) (* (Transformation|GetActorUpVector) (* _output_get (Variables|PhysicsValues|GetThrust%20Multiplier))) "None" true)
    (Development|PrintString (Utilities|String|ToString(Float) (* _output_get (Variables|PhysicsValues|GetThrust%20Multiplier))) true true "(R=1.000000,G=0.000000,B=0.780019,A=1.000000)" (Utilities|Time|GetWorldDeltaSeconds))))

(event Custom|Fuel%20Use
  (bind _output_get (Variables|Default|SetFuel (Math|Float|Clamp(Float) (- (Variables|Default|GetFuel) (* (Variables|Thrust|GetCurrent%20Thrust) (* (Variables|Default|GetFuel%20per%20Sec) (Variables|Default|GetFuelTick)))) 0.0 (Variables|Default|GetMax%20Fuel))))
  (Variables|Default|SetHas%20Fuel (> _output_get 0.0)))

(event Custom|Start%20Fuel%20Use
  (Utilities|Time|SetTimerbyEvent (delegate Custom|Fuel%20Use) (Variables|Default|GetFuelTick) true))

(event Input|ActionEvents|InputActionThrustUp
  (params (Key :type Key%20Structure))
  ;[1 1 1] Button Thrust input
  (:Pressed
    (Utilities|FlowControl|Sequence
      (:then_0
        (goto _label Open))
      (:then_1
        (Utilities|FlowControl|Gate true :!label _label
          (:Exit
            (Utilities|FlowControl|Sequence
              (:then_0
                (Utilities|FlowControl|Delay (Variables|Thrust|GetThrust%20Key%20Ticker))
                (goto _label))
              (:then_1
                (Variables|Thrust|SetTarget%20Thrust (Math|Float|Clamp(Float) (+ (Variables|Thrust|GetTarget%20Thrust) (Variables|Thrust|GetThrust%20Steps)))))))))))
  (:Released
    (goto _label Close)))

(event Input|ActionEvents|InputActionThrustDown
  (params (Key :type Key%20Structure))
  ;[1 1 1] Button Thrust input
  (:Pressed
    (Utilities|FlowControl|Sequence
      (:then_0
        (goto _label Open))
      (:then_1
        (Utilities|FlowControl|Gate true :!label _label
          (:Exit
            (Utilities|FlowControl|Sequence
              (:then_0
                (Utilities|FlowControl|Delay (Variables|Thrust|GetThrust%20Key%20Ticker))
                (goto _label))
              (:then_1
                (Variables|Thrust|SetTarget%20Thrust (Math|Float|Clamp(Float) (- (Variables|Thrust|GetTarget%20Thrust) (Variables|Thrust|GetThrust%20Steps)))))))))))
  (:Released
    (goto _label Close)))

(event Input|AxisEvents|InputAxisThrust
  (params (AxisValue :type Float%20%28single-precision%29))
  ;[1 1 1] Axis thrust input
  (if (Math|Float|NearlyEqual(Float) AxisValue 0.0 0.01)
    (Utilities|FlowControl|DoOnce false :!label _label
      (:Completed
        (Variables|Thrust|SetTarget%20Thrust 0.0)))
    (else
      (Utilities|FlowControl|Sequence
        (:then_0
          (goto _label Reset))
        (:then_1
          (Variables|Thrust|SetTarget%20Thrust AxisValue))))))

(event Input|AxisEvents|InputAxisPitch
  (params (AxisValue :type Float%20%28single-precision%29))
  ;[1 1 1] Rotation input. Pitch and yaw only fire if level is flagged 3d
  (if (Variables|Default|GetIs%203D?)
    (Class|PrimitiveComponent|AddTorqueinDegrees (Variables|Default|GetStaticMesh) (* (Transformation|GetActorRightVector) (* AxisValue (Variables|PhysicsValues|GetTorque))) "None" true)))

(event Input|AxisEvents|InputAxisYaw
  (params (AxisValue :type Float%20%28single-precision%29))
  ;[1 1 1] Rotation input. Pitch and yaw only fire if level is flagged 3d
  (if (Variables|Default|GetIs%203D?)
    (Class|PrimitiveComponent|AddTorqueinDegrees (Variables|Default|GetStaticMesh) (* (Transformation|GetActorUpVector) (* AxisValue (Variables|PhysicsValues|GetTorque))) "None" true)))

(event Input|AxisEvents|InputAxisRoll
  (params (AxisValue :type Float%20%28single-precision%29))
  ;[1 1 1] Rotation input. Pitch and yaw only fire if level is flagged 3d
  (Class|PrimitiveComponent|AddTorqueinDegrees (Variables|Default|GetStaticMesh) (* (Transformation|GetActorForwardVector) (* AxisValue (Variables|PhysicsValues|GetTorque))) "None" true))

(event Custom|Recieve%20Fuel
  (params (Value :type Float%20%28single-precision%29))
  (bind _output_get (Variables|Default|SetFuel (Math|Float|Clamp(Float) (+ Value (Variables|Default|GetFuel)) 0.0 (Variables|Default|GetMax%20Fuel))))
  (Development|PrintString (Utilities|String|ToString(Float) _output_get)))

(event Collision|EventHit
  (params (MyComp :type Primitive%20Component%20Object%20Reference) (Other :type Actor%20Object%20Reference) (OtherComp :type Primitive%20Component%20Object%20Reference) (bSelfMoved :type Boolean) (HitLocation :type Vector :default "0, 0, 0") (HitNormal :type Vector :default "0, 0, 0") (NormalImpulse :type Vector :default "0, 0, 0") (Hit :type Hit%20Result%20Structure%20%28by%20ref%29))
  (if (> (Math|Vector|VectorLength (Transformation|GetVelocity)) (Variables|Default|GetHit%20Tolerance))
    (Development|PrintString "you dead" true true "(R=1.000000,G=0.000000,B=0.063568,A=1.000000)" 2e+01)))

(fn ConstructionScript)