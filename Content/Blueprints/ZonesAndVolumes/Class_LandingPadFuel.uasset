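; Landing pad actor that refuels a Class_Lander while it sits inside the pad's box trigger.
; Entering the box stores the lander and enables fueling after a one-second delay, provided a lander is still stored and valid.
; A looping timer started at BeginPlay passes fuel rate times tick interval to the lander while fueling is on.
; Leaving the box stops fueling and clears the reference.
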(event OnComponentBeginOverlap(Box)
  (params (OverlappedComponent :type Primitive%20Component%20Object%20Reference) (OtherActor :type Actor%20Object%20Reference) (OtherComp :type Primitive%20Component%20Object%20Reference) (OtherBodyIndex :type Integer) (bFromSweep :type Boolean) (SweepResult :type Hit%20Result%20Structure%20%28by%20ref%29))
  (bind _asclass_lander (Utilities|Casting|CastToClass_Lander OtherActor)
    (:then
      (Variables|Default|SetLanderOnPad _asclass_lander)
      (CallFunction|Docked))
    (:CastFailed
      (Development|PrintString "fail"))))

(event OnComponentEndOverlap(Box)
  (params (OverlappedComponent :type Primitive%20Component%20Object%20Reference) (OtherActor :type Actor%20Object%20Reference) (OtherComp :type Primitive%20Component%20Object%20Reference) (OtherBodyIndex :type Integer))
  (if (== OtherActor (Variables|Default|GetLanderOnPad))
    (Variables|Default|SetFuel false)
    (Variables|Default|SetLanderOnPad 0)))

(event Custom|Docked
  (Utilities|FlowControl|Delay 1.0)
  (Utilities|IsValid (Variables|Default|GetLanderOnPad)
    (:Is%20Valid
      (Variables|Default|SetFuel true))))

(event Custom|Fueling
  (if (Variables|Default|GetFuel)
    (Default|RecieveFuel (Variables|Default|GetLanderOnPad) (* (Variables|Default|GetFuelRate) (Variables|Default|GetFuelTick)))
    (Development|PrintString "fuel")))

(event EventBeginPlay
  (Utilities|Time|SetTimerbyEvent (delegate Custom|Fueling) (Variables|Default|GetFuelTick) true))

(fn ConstructionScript)