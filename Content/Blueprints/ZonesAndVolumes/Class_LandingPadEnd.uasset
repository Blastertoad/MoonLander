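; Landing pad Blueprint that marks the end of a level and completes it when a lander docks.
; A box overlap stores the Class_Lander and starts Docked, which waits two seconds and checks that the stored lander is still valid.
; It then finds the current level name in GI_Lander's Levels array, sets the matching LevelsComplete entry to true, and calls Win on the game instance.
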(event OnComponentBeginOverlap(Box)
  (params (OverlappedComponent :type Primitive%20Component%20Object%20Reference) (OtherActor :type Actor%20Object%20Reference) (OtherComp :type Primitive%20Component%20Object%20Reference) (OtherBodyIndex :type Integer) (bFromSweep :type Boolean) (SweepResult :type Hit%20Result%20Structure%20%28by%20ref%29))
  (bind _asclass_lander (Utilities|Casting|CastToClass_Lander OtherActor))
  (Variables|Default|SetLanderOnPad _asclass_lander)
  (CallFunction|Docked))

(event Custom|Docked
  (Utilities|FlowControl|Delay 2.0)
  (Utilities|IsValid (Variables|Default|GetLanderOnPad)
    (:Is%20Valid
      (bind _returnvalue (Game|GetCurrentLevelName true))
      (bind _asgi_lander (Utilities|Casting|CastToGI_Lander (Game|GetGameInstance)))
      (Utilities|Array|SetArrayElem (Variables|/Game/Blueprints/Core/GI_Lander.GI_Lander_C|GetLevels%20Complete _asgi_lander) (Utilities|Array|FindItem (Variables|/Game/Blueprints/Core/GI_Lander.GI_Lander_C|GetLevels _asgi_lander) (Utilities|String|StringToName _returnvalue)) true)
      (Default|Win _asgi_lander))))

(fn ConstructionScript)